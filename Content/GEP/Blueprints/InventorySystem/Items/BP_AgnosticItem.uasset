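; BP_AgnosticItem is a generic dropped inventory item, shown in the world as a sprite of its item data's icon.
; On BeginPlay it keeps preset Data or, when the icon is unset, picks a random DataTable row.
; Each tick it bobs on a sine of its lifetime and yaws toward the player camera like a billboard.
; GetItemData exposes the data, and Pickup destroys the actor.
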(event `self.ReceiveBeginPlay`
  (bind (_data_name _data_description _data_stacksize _data_icon) (break `/Game/GEP/Blueprints/InventorySystem/F_ItemInfo` (`self.Data`)))
  (bind (_data_name_2 _data_description_2 _data_stacksize_2 _data_icon_2) (break `/Game/GEP/Blueprints/InventorySystem/F_ItemInfo` (`self.Data`)))
  ;[1 0.3385 0.6269] Displays set data or picks data at random for items
  (if (== _data_icon_2 null)
    (`self.GetRandomData`))
  (`PaperSpriteComponent.SetSprite` (`self.PaperSprite`) _data_icon))

(event `self.ReceiveTick`
  (params (DeltaSeconds :type "Float (single-precision)"))
  ;[1 0.417 0.2768] Dropped items bobble and face camera
  (`self.UpdateBobble`)
  (`self.FaceCamera`))

(event `/Game/GEP/Blueprints/Interfaces/BPI_Pickupable.Pickup`
  (`self.K2_DestroyActor`))

(fn `FaceCamera`
  (bind (_returnvalue_roll _returnvalue_pitch _returnvalue_yaw) (`KismetMathLibrary.BreakRotator` (`KismetMathLibrary.FindLookAtRotation` (`self.K2_GetActorLocation`) (`PlayerCameraManager.GetCameraLocation` (`GameplayStatics.GetPlayerCameraManager` 0)))))
  (`self.K2_SetActorRotation` (`KismetMathLibrary.MakeRotator` 0.0 0.0 _returnvalue_yaw)))

(fn `GetItemData`
  (returns (Data :type "/Game/GEP/Blueprints/InventorySystem/F_ItemInfo Structure"))
  (return (`self.Data`)))

(fn `GetRandomData`
  (bind _outrownames (`DataTableFunctionLibrary.GetDataTableRowNames` (`self.DataTable`)))
  (bind _returnvalue (`|GetDataTableRow` (`self.DataTable`) (`KismetArrayLibrary.Array_Random` _outrownames))
    (:`then`
      (set `self.Data` _returnvalue))))

(fn `UpdateBobble`
  (`SceneComponent.K2_AddRelativeLocation` (`self.DefaultSceneRoot`) (`KismetMathLibrary.MakeVector` 0.0 0.0 (* (`KismetMathLibrary.Sin` (* (`self.GetGameTimeSinceCreation`) (`self.BobbleSpeed`))) (`self.BobbleDistance`))) false false))

(fn `UserConstructionScript`)