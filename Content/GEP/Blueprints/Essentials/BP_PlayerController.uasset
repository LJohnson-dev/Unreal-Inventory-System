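; Player controller that sets up player input and owns the player menu widget used for the inventory.
; On BeginPlay it adds the player Enhanced Input mapping context, then creates the menu and adds it to the viewport hidden.
; The Inventory input shows and refreshes the menu, switches to UI-only input and shows the cursor; closing is not handled here.
; UpdateInventory re-runs the menu's Display to refresh it.
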(event `self.ReceiveBeginPlay`
  ;[1 1 1] Initialising the mapping context for the player input
  (`EnhancedInputSubsystemInterface.AddMappingContext` (subsystem `EnhancedInputLocalPlayerSubsystem`) "/Game/GEP/Input/IMC_Player.IMC_Player" 0 (struct))
  ;[1 1 1] Creating HUD and Menu widgets
  (bind _returnvalue (`|CreateWidget` "/Game/GEP/Blueprints/InventorySystem/UI/W_PlayerMenu.W_PlayerMenu_C"))
  (set `self.Menu` _returnvalue)
  (`UserWidget.AddToViewport` (`self.Menu`) 0)
  (`Widget.SetVisibility` (`self.Menu`) "Hidden"))

(event `InputAction|Inventory`
  (params (Key :type "Key Structure"))
  (bind _menu (`self.Menu`))
  ;[1 1 1] Toggling Inventory visibility based on input action
  (:`Pressed`
    (`Widget.SetVisibility` _menu "Visible")
    (`/Game/GEP/Blueprints/InventorySystem/UI/W_PlayerMenu.Display` _menu)
    (`WidgetBlueprintLibrary.SetInputMode_UIOnlyEx` (`GameplayStatics.GetPlayerController` 0) (`self.Menu`))
    (set `self.bShowMouseCursor` true)))

(fn `UpdateInventory`
  (`/Game/GEP/Blueprints/InventorySystem/UI/W_PlayerMenu.Display` (`self.Menu`)))

(fn `UserConstructionScript`)